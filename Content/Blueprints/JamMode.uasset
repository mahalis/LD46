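; JamMode is the game mode that runs a level's flow from title through play to end screen, tracking score.
; On BeginPlay it creates the UI widgets, finds or spawns a CountdownController and reads LevelInfoContainer, auto-starting non-intro levels.
; Begin, End and Reset toggle widgets and play state.
; Retry clears Aquarium and LostFish actors and possesses a fresh pawn at PlayerStart without reloading, while next level opens by name.
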(event `self.ReceiveBeginPlay`
  (`WidgetBlueprintLibrary.SetFocusToGameViewport`)
  (`|ExecutionSequence`
    (:`then_0`
      (`WidgetBlueprintLibrary.SetInputMode_GameAndUIEx` (`GameplayStatics.GetPlayerController` 0) null "LockOnCapture" false))
    (:`then_1`
      (`self.SetupUI`))
    (:`then_2`
      (bind _outactors (`GameplayStatics.GetAllActorsOfClass` "/Game/Blueprints/World/CountdownController.CountdownController_C"))
      (if (> (`KismetArrayLibrary.Array_Length` _outactors) 0)
        (set `self.CounterDown` (`|GetArrayItem` _outactors))
        (else
          (bind _returnvalue (`|SpawnActorFromClass` "/Game/Blueprints/World/CountdownController.CountdownController_C" (`KismetMathLibrary.MakeTransform` (0.0 0.0 0.0)) "AlwaysSpawn" "OverrideRootScale" null null))
          (set `self.CounterDown` _returnvalue))))
    (:`then_3`
      (bind _outactors_2 (`GameplayStatics.GetAllActorsOfClass` "/Game/Blueprints/LevelInfoContainer.LevelInfoContainer_C"))
      (bind _output (`|GetArrayItem` _outactors_2))
      (set `self.NextLevelName` (`/Game/Blueprints/LevelInfoContainer.NextLevelName` _output))
      (set `self.IsIntroLevel` (`/Game/Blueprints/LevelInfoContainer.IsIntro` _output)))
    (:`then_4`
      (`self.Reset`)
      (if (not (`self.IsIntroLevel`))
        (`self.Begin`)))))

(fn `AddScore`
  (params (Amount :type Integer))
  (set `self.Score` (+ (`self.Score`) Amount)))

(fn `Begin`
  (bind _counterdown (`self.CounterDown`))
  (set `self.Playing` true)
  (`Widget.SetVisibility` (`self.TitleScreenWidget`) "Hidden")
  (`Widget.SetVisibility` (`self.HUDWidget`) "Visible")
  (`Widget.SetVisibility` (`self.InstructionWidget`) "Visible")
  (`Widget.SetVisibility` (`self.LevelEndScreenWidget`) "Hidden")
  (`WidgetBlueprintLibrary.SetInputMode_GameOnly` (`GameplayStatics.GetPlayerController` 0))
  (if (`/Game/Blueprints/World/CountdownController.StartAutomatically` _counterdown)
    (`/Game/Blueprints/World/CountdownController.BeginCountdown` _counterdown)))

(fn `End`
  (set `self.Playing` false)
  (set `self.GameOver` true)
  (`Widget.SetVisibility` (`self.LevelEndScreenWidget`) "Visible")
  (`Widget.SetVisibility` (`self.HUDWidget`) "Hidden")
  (`/Game/Blueprints/UI/LevelCompleteScreen.SetResult` (`self.LevelEndScreenWidget`) (`self.Score`) (!= (`self.NextLevelName`) "None") (`self.HasEverUsedGamepad`))
  (`GameplayStatics.PlaySound2D` "/Game/Sounds/LevelEnd.LevelEnd" 1.0 1.0 0.0 null null))

(fn `GetCurrentInstruction`
  (returns (Instruction :type "/Game/Blueprints/UI/InstructionState Enum") (CustomText :type String))
  (bind (_state _customtext) (`/Game/Blueprints/UI/Instructions.GetState` (`self.InstructionWidget`)))
  (return _state _customtext))

(fn `GetScore`
  (returns (Score :type Integer))
  (return (`self.Score`)))

(fn `RequestNextLevel`
  (`GameplayStatics.OpenLevel` (`self.NextLevelName`)))

(fn `RequestRetryLevel`
  (bind _returnvalue (`GameplayStatics.GetPlayerController` 0))
  (`self.Reset`)
  (bind _outactors (`GameplayStatics.GetAllActorsOfClass` "/Script/Engine.PlayerStart"))
  (bind _returnvalue_2 (`|SpawnActorFromClass` "/Game/Blueprints/Player/RollerPawn.RollerPawn_C" (`self.GetTransform` (`|GetArrayItem` _outactors)) "AdjustIfPossibleButAlwaysSpawn" "OverrideRootScale" null null))
  (`self.K2_DestroyActor` (`Controller.K2_GetPawn` _returnvalue))
  (`Controller.Possess` _returnvalue _returnvalue_2)
  (`self.SetCurrentInstruction` "NewEnumerator0")
  (`self.Begin`))

(fn `Reset`
  (set `self.Playing` false)
  (set `self.GameOver` false)
  (`Widget.SetVisibility` (`self.HUDWidget`) "Hidden")
  (`Widget.SetVisibility` (`self.LevelEndScreenWidget`) "Hidden")
  (set `self.Score` 0)
  (`WidgetBlueprintLibrary.SetInputMode_UIOnlyEx` (`GameplayStatics.GetPlayerController` 0) null)
  (`Widget.SetVisibility` (`self.InstructionWidget`) "Hidden")
  (bind _outactors (`GameplayStatics.GetAllActorsOfClass` "/Game/Blueprints/Aquarium.Aquarium_C"))
  (for _array_element _outactors
    (`self.K2_DestroyActor` _array_element))
  (bind _outactors_2 (`GameplayStatics.GetAllActorsOfClass` "/Game/Blueprints/LostFish.LostFish_C"))
  (for _array_element_2 _outactors_2
    (`self.K2_DestroyActor` _array_element_2)))

(fn `SetCurrentInstruction`
  (params (State :type "/Game/Blueprints/UI/InstructionState Enum" :default "NewEnumerator0") (CustomText :type String))
  (`/Game/Blueprints/UI/Instructions.SetState` (`self.InstructionWidget`) State CustomText false))

(fn `SetupUI`
  (bind _returnvalue (`GameplayStatics.GetPlayerController` 0))
  (`|ExecutionSequence`
    (:`then_0`
      (bind _returnvalue_2 (`|CreateWidget` "/Game/Blueprints/UI/TitleScreen.TitleScreen_C" _returnvalue))
      (bind _output_get (set `self.TitleScreenWidget` _returnvalue_2))
      (`UserWidget.AddToViewport` _output_get 3))
    (:`then_1`
      (bind _returnvalue_3 (`|CreateWidget` "/Game/Blueprints/UI/JamHUD.JamHUD_C" _returnvalue))
      (bind _output_get_2 (set `self.HUDWidget` _returnvalue_3))
      (`UserWidget.AddToViewport` _output_get_2 0))
    (:`then_2`
      (bind _returnvalue_4 (`|CreateWidget` "/Game/Blueprints/UI/Instructions.Instructions_C" _returnvalue))
      (bind _output_get_3 (set `self.InstructionWidget` _returnvalue_4))
      (`UserWidget.AddToViewport` _output_get_3 1))
    (:`then_3`
      (bind _returnvalue_5 (`|CreateWidget` "/Game/Blueprints/UI/LevelCompleteScreen.LevelCompleteScreen_C" _returnvalue))
      (bind _output_get_4 (set `self.LevelEndScreenWidget` _returnvalue_5))
      (`UserWidget.AddToViewport` _output_get_4 2))))

(fn `UserConstructionScript`)