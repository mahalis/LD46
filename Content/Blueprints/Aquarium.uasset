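; Physics-simulated aquarium actor that spills its fish when it tips over.
; Construction sizes the box and enables physics, and the first hit on a landscape or static mesh actor marks it as landed.
; Tick watches the up vector and, past about 60 degrees of tilt, hides water and fish, launches a spawned LostFish along the tank's up axis with random spread, then stops ticking.
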(event `self.ReceiveTick`
  (params (DeltaSeconds :type "Float (single-precision)"))
  (if (< (`KismetMathLibrary.Dot_VectorVector` (`self.GetActorUpVector`) (0.0 0.0 1.0)) 0.5)
    (`self.Fell`)
    (`self.SetActorTickEnabled` false)))

(event `self.ReceiveHit`
  (params (MyComp :type "PrimitiveComponent Object Reference") (Other :type "Actor Object Reference") (OtherComp :type "PrimitiveComponent Object Reference") (bSelfMoved :type Boolean) (HitLocation :type "Vector Structure") (HitNormal :type "Vector Structure") (NormalImpulse :type "Vector Structure") (Hit :type "HitResult Structure (by ref)"))
  (if (not (`self.HasLanded`))
    (cast `Landscape` Other
      (:`then`
        _)
      (:`CastFailed`
        (cast `StaticMeshActor` Other)))
    (`self.Landed`)))

(fn `Fell`
  (bind _fish (`self.Fish`))
  (`SceneComponent.SetHiddenInGame` (`self.Water`) true true)
  (`SceneComponent.SetHiddenInGame` _fish true false)
  (bind _returnvalue (`|SpawnActorFromClass` "/Game/Blueprints/LostFish.LostFish_C" (`SceneComponent.K2_GetComponentToWorld` _fish) "AlwaysSpawn" "OverrideRootScale" null null))
  (`PrimitiveComponent.AddImpulse` (`/Game/Blueprints/LostFish.Mesh` _returnvalue) (* (`KismetMathLibrary.RandomUnitVectorInConeInDegrees` (`self.GetActorUpVector`) 20.0) (`KismetMathLibrary.RandomFloatInRange` 150.0 250.0)) "None" true))

(fn `GetAxes`
  (returns (Forward :type "Vector2D Structure") (Right :type "Vector2D Structure"))
  (bind (_returnvalue_x _returnvalue_y) (`KismetMathLibrary.BreakVector` (`self.GetActorRightVector`)))
  (bind (_returnvalue_x_2 _returnvalue_y_2) (`KismetMathLibrary.BreakVector` (`self.GetActorForwardVector`)))
  (return (`KismetMathLibrary.Normal2D` (`KismetMathLibrary.MakeVector2D` _returnvalue_x_2 _returnvalue_y_2)) (`KismetMathLibrary.Normal2D` (`KismetMathLibrary.MakeVector2D` _returnvalue_x _returnvalue_y))))

(fn `Landed`
  (set `self.HasLanded` true))

(fn `UserConstructionScript`
  (bind _box (`self.Box`))
  (`BoxComponent.SetBoxExtent` _box (`self.Size`) true)
  (`PrimitiveComponent.SetSimulatePhysics` _box true))