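; Player platform that carries Aquariums between a pickup zone and a dropoff zone.
; A constraint keeps it level and turned to the controller's yaw, while an arrow smoothly points to pickup, or to dropoff when carrying.
; CarryDetector overlaps set the carrying state.
; Losing the last Aquarium prints a happy or sad reaction, depending on a success flag that NotifySuccessfulDropoff raises and a one-second timer clears.
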(event `self.ReceiveBeginPlay`
  (bind _outactors (`GameplayStatics.GetAllActorsOfClass` "/Game/Blueprints/World/PickupZone.PickupZone_C"))
  (set `self.PickupLocation` (`self.K2_GetActorLocation` (`|GetArrayItem` _outactors)))
  (bind _outactors_2 (`GameplayStatics.GetAllActorsOfClass` "/Game/Blueprints/World/DropoffZone.DropoffZone_C"))
  (set `self.DropoffLocation` (`self.K2_GetActorLocation` (`|GetArrayItem` _outactors_2))))

(event `self.ReceiveTick`
  (params (DeltaSeconds :type "Float (single-precision)"))
  (bind (_returnvalue_roll _returnvalue_pitch _returnvalue_yaw) (`KismetMathLibrary.BreakRotator` (`Controller.GetControlRotation` (`GameplayStatics.GetPlayerController` 0))))
  (`PhysicsConstraintComponent.SetAngularOrientationTarget` (`self.Uprightness`) (`KismetMathLibrary.MakeRotator` 0.0 0.0 _returnvalue_yaw))
  (`self.UpdateNavigationArrow` DeltaSeconds))

(event `self.CarryDetector.OnComponentBeginOverlap`
  (params (OverlappedComponent :type "PrimitiveComponent Object Reference") (OtherActor :type "Actor Object Reference") (OtherComp :type "PrimitiveComponent Object Reference") (OtherBodyIndex :type Integer) (bFromSweep :type Boolean) (SweepResult :type "HitResult Structure (by ref)"))
  (cast `/Game/Blueprints/Aquarium` OtherActor)
  (`self.SetCarrying` true))

(event `self.CarryDetector.OnComponentEndOverlap`
  (params (OverlappedComponent :type "PrimitiveComponent Object Reference") (OtherActor :type "Actor Object Reference") (OtherComp :type "PrimitiveComponent Object Reference") (OtherBodyIndex :type Integer))
  (cast `/Game/Blueprints/Aquarium` OtherActor)
  (if (== (`KismetArrayLibrary.Array_Length` (`PrimitiveComponent.GetOverlappingActors` (`self.CarryDetector`) "/Game/Blueprints/Aquarium.Aquarium_C")) 0)
    (`self.SetCarrying` false)))

(fn `NotifySuccessfulDropoff`
  (set `self.JustSucceeded` true)
  (`KismetSystemLibrary.K2_SetTimer` null "ResetReaction" 1.0))

(fn `ReactToNotCarrying`
  (if (`self.JustSucceeded`)
    (`KismetSystemLibrary.PrintString` "yay!")
    (else
      (`KismetSystemLibrary.PrintString` ":("))))

(fn `ResetReaction`
  (set `self.JustSucceeded` false))

(fn `SetCarrying`
  (params (NewCarrying :type Boolean))
  (if (!= (`self.Carrying`) NewCarrying)
    (if (not NewCarrying)
      (`self.ReactToNotCarrying`))
    (set `self.Carrying` NewCarrying)))

(fn `UpdateNavigationArrow`
  (params (DeltaTime :type "Float (double-precision)"))
  (bind _navigationarrow (`self.NavigationArrow`))
  (bind _returnvalue (- (`KismetMathLibrary.SelectVector` (`self.DropoffLocation`) (`self.PickupLocation`) (`self.Carrying`)) (`SceneComponent.K2_GetComponentLocation` (`self.NavigationArrow`))))
  (if (> (`KismetMathLibrary.VSizeSquared` _returnvalue) 400.0)
    (`SceneComponent.K2_SetWorldRotation` _navigationarrow (`KismetMathLibrary.RInterpTo` (`SceneComponent.K2_GetComponentRotation` _navigationarrow) (`KismetMathLibrary.MakeRotator` 0.0 0.0 (+ (`KismetMathLibrary.DegAtan2` (.y _returnvalue) (.x _returnvalue)) -90.0)) DeltaTime 5.0) false false)))

(fn `UserConstructionScript`)