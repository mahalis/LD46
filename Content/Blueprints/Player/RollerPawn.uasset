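; RollerPawn is a player pawn that rolls a physics sphere carrying a separately spawned Platform actor.
; On BeginPlay it spawns the Platform above itself and binds it to the sphere through the PlatformLock constraint, destroying it with the pawn.
; Each tick, clamped movement input becomes a yaw-relative, delta-scaled impulse on the sphere, while turn axes drive controller yaw.
; AddAquarium registers aquariums in the Aquaria collection.
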(event `self.ReceiveBeginPlay`
  (bind _returnvalue (`self.GetTransform`))
  (bind _returnvalue_2 (`|SpawnActorFromClass` "/Game/Blueprints/Player/Platform.Platform_C" (`KismetMathLibrary.MakeTransform` (`KismetMathLibrary.MakeVector` (.x (.location _returnvalue)) (.y (.location _returnvalue)) (+ (.z (.location _returnvalue)) 96.0))) "Undefined" "OverrideRootScale" null null))
  (set `self.Platform` _returnvalue_2)
  (`PhysicsConstraintComponent.SetConstrainedComponents` (`self.PlatformLock`) (`self.Sphere`) "None" (`/Game/Blueprints/Player/Platform.PlatformCollision` _returnvalue_2) "None"))

(event `InputAxis|TurnRate`
  (params (AxisValue :type "Float (single-precision)"))
  (`self.AddControllerYawInput` (* AxisValue (`GameplayStatics.GetWorldDeltaSeconds`) 40.0)))

(event `InputAxis|Turn` :overrideparent false
  (params (AxisValue :type "Float (single-precision)"))
  (`self.AddControllerYawInput` (* AxisValue 0.6)))

(event `self.ReceiveTick`
  (params (DeltaSeconds :type "Float (single-precision)"))
  (`self.ApplyMovement` DeltaSeconds))

(event `self.ReceiveDestroyed`
  (`self.K2_DestroyActor` (`self.Platform`)))

(fn `AddAquarium`
  (params (NewAquarium :type "/Game/Blueprints/Aquarium Object Reference"))
  (`KismetArrayLibrary.Array_Add` (`self.Aquaria`) NewAquarium))

(fn `ApplyMovement`
  (params (DeltaTime :type "Float (double-precision)"))
  (bind (_returnvalue_roll _returnvalue_pitch _returnvalue_yaw) (`KismetMathLibrary.BreakRotator` (`self.GetBaseAimRotation`)))
  (bind (_forward _right) (`self.ReasonableMovementVector`))
  (bind _returnvalue (`KismetMathLibrary.DegCos` _returnvalue_yaw))
  (bind _returnvalue_2 (`KismetMathLibrary.DegSin` _returnvalue_yaw))
  (`PrimitiveComponent.AddImpulse` (`self.Sphere`) (* (+ (* (`KismetMathLibrary.MakeVector` _returnvalue _returnvalue_2) _forward) (* (`KismetMathLibrary.MakeVector` (* _returnvalue_2 -1.0) _returnvalue) _right)) (* 280000.0 DeltaTime)) "None" false))

(fn `ReasonableMovementVector`
  (returns (Forward :type "Float (double-precision)") (Right :type "Float (double-precision)"))
  (bind _returnvalue (`KismetMathLibrary.MakeVector2D` (`self.GetInputAxisValue`) (`self.GetInputAxisValue`)))
  (bind _returnvalue_2 (`KismetMathLibrary.VSize2DSquared` _returnvalue))
  (bind (_returnvalue_x _returnvalue_y) (`KismetMathLibrary.BreakVector2D` (select `bool` (> _returnvalue_2 1.0) :`false` _returnvalue :`true` (/ _returnvalue (`KismetMathLibrary.Sqrt` _returnvalue_2)))))
  (return _returnvalue_y _returnvalue_x))

(fn `UserConstructionScript`)