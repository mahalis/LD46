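; Pickup zone that spawns Aquarium cargo onto a RollerPawn inside it and drives pickup instructions through JamMode.
; Overlap toggles Tick, which polls the pawn's WantsProvision against a timer-reset cooldown.
; A downward sphere trace finds the top of the load, skipping overcrowded spots, and spawns an aquarium there with randomized placement.
; Instructions show immediately in introduction zones, otherwise after a delay, and advance on pickup or introduction-zone exit.
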(event `self.ReceiveBeginPlay`
  (bind _asjam_mode (cast `/Game/Blueprints/JamMode` (`GameplayStatics.GetGameMode`)))
  (set `self.Mode` _asjam_mode))

(event `self.ReceiveActorBeginOverlap`
  (params (OtherActor :type "Actor Object Reference"))
  (bind _asroller_pawn (cast `/Game/Blueprints/Player/RollerPawn` OtherActor))
  (set `self.Pawn` _asroller_pawn)
  (`self.SetActorTickEnabled` true)
  (if (`self.IsIntroduction`)
    (`self.ShowInstructions`)
    (else
      (`KismetSystemLibrary.K2_SetTimer` null "DelayedShowInstructions" 1.0))))

(event `self.ReceiveActorEndOverlap`
  (params (OtherActor :type "Actor Object Reference"))
  (cast `/Game/Blueprints/Player/RollerPawn` OtherActor)
  (set `self.Pawn` null)
  (`self.SetActorTickEnabled` false)
  (`KismetSystemLibrary.K2_ClearTimer` null "DelayedShowInstructions")
  (`KismetSystemLibrary.K2_SetTimer` null "ResetCanProvide" 0.2)
  (`self.ConsiderShowingDeliveryInstruction`))

(event `self.ReceiveTick`
  (params (DeltaSeconds :type "Float (single-precision)"))
  (bind _pawn (`self.Pawn`))
  (`/Engine/EditorBlueprintResources/StandardMacros.IsValid` _pawn
    (:`Is Valid`
      (bind _did (`self.ConsiderProvision` _pawn))
      (if _did
        (`KismetSystemLibrary.K2_SetTimer` null "ResetCanProvide" 1.5)))))

(fn `ConsiderProvision`
  (params (To :type "/Game/Blueprints/Player/RollerPawn Object Reference"))
  (returns (Did :type Boolean))
  (locals (NewAquariumWidth :type "Float (double-precision)") (NewAquariumDepth :type "Float (double-precision)") (NewAquariumHeight :type "Float (double-precision)") (PlacementHeight :type "Float (double-precision)" :default 0.0))
  (bind _returnvalue (`self.K2_GetActorLocation` To))
  (bind (_returnvalue_x _returnvalue_y) (`KismetMathLibrary.BreakVector` (+ _returnvalue (`KismetMathLibrary.RandomPointInBoundingBox` (0.0 0.0 0.0) (10.0 10.0 0.0)))))
  (if (and (`/Game/Blueprints/Player/RollerPawn.WantsProvision` To) (`self.CanProvide`))
    (bind (_outhit _returnvalue_2) (`KismetSystemLibrary.SphereTraceSingleForObjects` (+ _returnvalue (0.0 0.0 600.0)) _returnvalue 50.0 (`|MakeArray` "ObjectTypeQuery4" "ObjectTypeQuery3" :!type "EObjectTypeQuery Enum")))
    (if _returnvalue_2
      (set `self.CanProvide` false)
      (if (`.bInitialOverlap` (`GameplayStatics.BreakHitResult` _outhit))
        (return false)
        (else
          (set `local.PlacementHeight` (.z (`.ImpactPoint` (`GameplayStatics.BreakHitResult` _outhit))))
          (`|SpawnActorFromClass` "/Game/Blueprints/Aquarium.Aquarium_C" (`KismetMathLibrary.MakeTransform` (`KismetMathLibrary.MakeVector` _returnvalue_x _returnvalue_y (+ (`local.PlacementHeight`) 30.0)) (`KismetMathLibrary.MakeRotator` 0.0 0.0 (`KismetMathLibrary.RandomFloatInRange` 0.0 360.0)) (`KismetMathLibrary.MakeVector` (`KismetMathLibrary.RandomFloatInRange` 1.0 1.1) 1.0 (`KismetMathLibrary.RandomFloatInRange` 0.9 1.0))) "AdjustIfPossibleButAlwaysSpawn" "OverrideRootScale" null null)
          (`KismetSystemLibrary.K2_SetTimer` null "ResetCanProvide" 0.5)
          (bind _instruction (`/Game/Blueprints/JamMode.GetCurrentInstruction` (`self.Mode`)))
          (if (`|EnumEquality` _instruction "NewEnumerator3")
            (`/Game/Blueprints/JamMode.SetCurrentInstruction` (`self.Mode`) "NewEnumerator5" "(You can carry more than one!)"))
          (return true)))
      (else
        (return false)))
    (else
      (return false))))

(fn `ConsiderShowingDeliveryInstruction`
  (if (`self.IsIntroduction`)
    (`/Game/Blueprints/JamMode.SetCurrentInstruction` (`self.Mode`) "NewEnumerator4" "")))

(fn `DelayedShowInstructions`
  (if (> (`KismetArrayLibrary.Array_Length` (`self.GetOverlappingActors` "/Game/Blueprints/Player/RollerPawn.RollerPawn_C")) 0)
    (`self.ShowInstructions`)))

(fn `ResetCanProvide`
  (set `self.CanProvide` true))

(fn `ShowInstructions`
  (`/Game/Blueprints/JamMode.SetCurrentInstruction` (`self.Mode`) "NewEnumerator3" ""))

(fn `UserConstructionScript`)