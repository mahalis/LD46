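; DropoffZone is a delivery point where the RollerPawn drops off Aquarium actors for score.
; Pawn overlap toggles Tick, which checks whether the pawn is near the zone's centre in 2D.
; It then gathers aquaria overlapping the capsule, adds score to JamMode from a count-indexed table, and destroys them.
; Introduction zones also show a congratulation through JamMode, followed by a timed instruction about the 60-second challenge.
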(event `self.ReceiveBeginPlay`
  (bind _asjam_mode (cast `/Game/Blueprints/JamMode` (`GameplayStatics.GetGameMode`)))
  (set `self.Mode` _asjam_mode))

(event `self.ReceiveActorBeginOverlap`
  (params (OtherActor :type "Actor Object Reference"))
  (bind _asroller_pawn (cast `/Game/Blueprints/Player/RollerPawn` OtherActor))
  (set `self.Pawn` _asroller_pawn)
  (`self.SetActorTickEnabled` true))

(event `self.ReceiveTick`
  (params (DeltaSeconds :type "Float (single-precision)"))
  (`self.ConsiderAcquiringAquaria`))

(event `self.ReceiveActorEndOverlap`
  (params (OtherActor :type "Actor Object Reference"))
  (cast `/Game/Blueprints/Player/RollerPawn` OtherActor)
  (`self.SetActorTickEnabled` false))

(fn `ConsiderAcquiringAquaria`
  (locals (AquariaToAcquire :type "Array of /Game/Blueprints/Aquarium Object Reference"))
  (bind _returnvalue (`KismetArrayLibrary.Array_Length` (`local.AquariaToAcquire`)))
  (if (< (`KismetMathLibrary.Vector_Distance2DSquared` (`self.K2_GetActorLocation`) (`self.K2_GetActorLocation` (`self.Pawn`))) 900.0)
    (for _array_element (`PrimitiveComponent.GetOverlappingActors` (`self.Capsule`) "/Game/Blueprints/Aquarium.Aquarium_C")
      (bind _asaquarium (cast `/Game/Blueprints/Aquarium` _array_element))
      (`/Engine/EditorBlueprintResources/StandardMacros.IsValid` _asaquarium
        (:`Is Valid`
          (`KismetArrayLibrary.Array_Add` (`local.AquariaToAcquire`) _asaquarium))))
    (if (> _returnvalue 0)
      (bind _asjam_mode (cast `/Game/Blueprints/JamMode` (`GameplayStatics.GetGameMode`)))
      (`/Game/Blueprints/JamMode.AddScore` _asjam_mode (select `int` _returnvalue :`0` 0 :`1` 2 :`2` 8 :`3` 16 :`4` 12))
      (`self.ConsiderCongratulating`)
      (for _array_element_2 (`local.AquariaToAcquire`)
        (`self.K2_DestroyActor` _array_element_2)))))

(fn `ConsiderCongratulating`
  (if (and (`self.IsIntroduction`) (not (`self.HasCongratulated`)))
    (`/Game/Blueprints/JamMode.SetCurrentInstruction` (`self.Mode`) "NewEnumerator5" "Good job!")
    (`KismetSystemLibrary.K2_SetTimer` null "DelayedInstructTimer" 2.0)))

(fn `DelayedInstructTimer`
  (`/Game/Blueprints/JamMode.SetCurrentInstruction` (`self.Mode`) "NewEnumerator5" "Deliver as many as you can in 60 seconds!"))

(fn `UserConstructionScript`)