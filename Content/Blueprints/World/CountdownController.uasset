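; CountdownController is an actor that runs a pre-start countdown and then a round timer through the JamMode game mode.
; BeginCountdown shows a three-second countdown as instruction text, then displays "Go!" and starts the timer from InitialTime.
; Both phases tick once per second by re-arming a timer by function name, with remaining time pushed to the mode's HUD widget.
; Reaching zero only prints an out-of-time debug message.
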(event `self.ReceiveBeginPlay`
  (bind _asjam_mode (cast `/Game/Blueprints/JamMode` (`GameplayStatics.GetGameMode`)))
  (set `self.Mode` _asjam_mode))

(fn `AdvanceCountdown`
  (bind _countdownremaining (`self.CountdownRemaining`))
  (if (> _countdownremaining 0)
    (`/Game/Blueprints/JamMode.SetCurrentInstruction` (`self.Mode`) "NewEnumerator5" (`KismetStringLibrary.BuildString_Int` "" "" _countdownremaining "…"))
    (set `self.CountdownRemaining` (- _countdownremaining 1))
    (`KismetSystemLibrary.K2_SetTimer` null "AdvanceCountdown" 1.0)
    (else
      (`self.BeginTime`))))

(fn `AdvanceTime`
  (bind _remainingtime (`self.RemainingTime`))
  (`/Game/Blueprints/UI/JamHUD.SetRemainingTime` (`/Game/Blueprints/JamMode.HUDWidget` (`self.Mode`)) _remainingtime)
  (if (> _remainingtime 0)
    (set `self.RemainingTime` (- _remainingtime 1))
    (`KismetSystemLibrary.K2_SetTimer` null "AdvanceTime" 1.0)
    (else
      (`KismetSystemLibrary.PrintString` "out of time!"))))

(fn `BeginCountdown`
  (set `self.CountdownRemaining` 3)
  (`self.AdvanceCountdown`))

(fn `BeginTime`
  (`/Game/Blueprints/JamMode.SetCurrentInstruction` (`self.Mode`) "NewEnumerator5" "Go!")
  (set `self.RemainingTime` (`self.InitialTime`))
  (`self.AdvanceTime`))

(fn `UserConstructionScript`)